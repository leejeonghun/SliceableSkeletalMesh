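; Character whose body is built from static meshes named after skeleton bones, which can be sliced apart at a given point with a visible guideline.
; The first cut on a part converts it to a capped procedural mesh, ragdolls the body, and reattaches halves via a parent-bone search, breaking the constraint when a parent static mesh exists.
; Later cuts re-slice procedural pieces, orienting the plane by hierarchy so the new half simulates physics and carries child pieces.
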(fn `FindParentBoneMesh`
  (params (BoneName :type Name))
  (returns (ReturnValue :type "StaticMeshComponent Object Reference") (ParentBoneName :type Name))
  (locals (FindBoneMesh :type "StaticMeshComponent Object Reference") (FindBoneName :type Name))
  (bind _returnvalue (`SkinnedMeshComponent.GetParentBone` (`self.Mesh`) (`local.FindBoneName`)))
  (set `local.FindBoneName` BoneName)
  (if (!= _returnvalue "None") :!label _label
    (bind _output_get (set `local.FindBoneName` _returnvalue))
    (bind _returnvalue_2 (`self.FindStaticMeshByBoneName` _output_get))
    (`/Engine/EditorBlueprintResources/StandardMacros.IsValid` _returnvalue_2
      (:`Is Valid`
        (return _returnvalue_2 (`local.FindBoneName`)))
      (:`Is Not Valid`
        (if (`BlueprintMapLibrary.Map_Contains` (`self.ProcMeshMap`) (`local.FindBoneName`))
          (return null (`local.FindBoneName`))
          (else
            (goto _label)))))
    (else
      (return null "None"))))

(fn `FindStaticMeshByBoneName`
  (params (BoneName :type Name))
  (returns (ReturnValue :type "StaticMeshComponent Object Reference"))
  (locals (FindBoneMesh :type "StaticMeshComponent Object Reference"))
  (for _array_element (`SceneComponent.GetChildrenComponents` (`self.Mesh`) false)
    (bind _asstatic_mesh_component (cast `StaticMeshComponent` _array_element))
    (if (== (`local.BoneName`) (`KismetStringLibrary.Conv_StringToName` (`KismetStringLibrary.ToLower` (`KismetSystemLibrary.GetObjectName` _asstatic_mesh_component))))
      (set `local.FindBoneMesh` _asstatic_mesh_component)
      (break)))
  (return (`local.FindBoneMesh`)))

(fn `ShowSliceGuideline`
  (params (Location :type "Vector Structure") (Component :type "PrimitiveComponent Object Reference") (Hide :type Boolean))
  (locals (Bounds :type "Vector Structure" :default (0.0 0.0 0.0)) (Normal :type "Vector Structure" :default (0.0 0.0 0.0)) (Center :type "Vector Structure" :default (0.0 0.0 0.0)))
  (bind (_bounds_x _bounds_y _bounds_z) (`KismetMathLibrary.BreakVector` (`local.Bounds`)))
  (bind _returnvalue (`SceneComponent.K2_GetComponentToWorld` (`local.Component`)))
  (bind _returnvalue_2 (`StaticMesh.GetBounds` (`StaticMeshComponent.StaticMesh` (`self.Guideline`))))
  (bind (_returnvalue_x _returnvalue_y _returnvalue_z) (`KismetMathLibrary.BreakVector` (`KismetMathLibrary.InverseTransformLocation` _returnvalue (`local.Center`))))
  (bind _returnvalue_x_2 (`KismetMathLibrary.BreakVector` (`KismetMathLibrary.InverseTransformLocation` _returnvalue (`local.Location`))))
  (`SceneComponent.SetVisibility` (`self.Guideline`) (not Hide) false)
  (bind _asstatic_mesh_component (cast `StaticMeshComponent` Component)
    (:`then`
      (set `local.Center` (`KismetSystemLibrary.GetComponentBounds` _asstatic_mesh_component))
      (bind (_returnvalue_origin _returnvalue_boxextent) (`KismetMathLibrary.BreakBoxSphereBounds` (`StaticMesh.GetBounds` (`StaticMeshComponent.StaticMesh` _asstatic_mesh_component))))
      (set `local.Bounds` _returnvalue_boxextent))
    (:`CastFailed`
      (bind _asprocedural_mesh_component (cast `ProceduralMeshComponent` (`local.Component`)))
      (bind (_origin _boxextent) (`KismetSystemLibrary.GetComponentBounds` _asprocedural_mesh_component))
      (set `local.Center` _origin)
      (set `local.Bounds` _boxextent)))
  (`SceneComponent.K2_SetWorldTransform` (`self.Guideline`) (`KismetMathLibrary.MakeTransform` (`KismetMathLibrary.TransformLocation` _returnvalue (`KismetMathLibrary.MakeVector` _returnvalue_x_2 _returnvalue_y _returnvalue_z)) (`SceneComponent.K2_GetComponentRotation` (`local.Component`))) false true)
  (`SceneComponent.K2_AddLocalRotation` (`self.Guideline`) (`KismetMathLibrary.RotatorFromAxisAndAngle` (0.0 1.0 0.0) 90.0) false false)
  (`SceneComponent.SetWorldScale3D` (`self.Guideline`) (`KismetMathLibrary.MakeVector` (* (/ _bounds_z (.y (`.BoxExtent` (`KismetMathLibrary.BreakBoxSphereBounds` _returnvalue_2)))) 1.05) (* (/ _bounds_y (.x (`.BoxExtent` (`KismetMathLibrary.BreakBoxSphereBounds` _returnvalue_2)))) 1.05) 1.0)))

(fn `Slice`
  (params (Location :type "Vector Structure") (Component :type "PrimitiveComponent Object Reference"))
  (bind _location (`local.Location`))
  (bind _returnvalue (`KismetMathLibrary.GetForwardVector` (`SceneComponent.K2_GetComponentRotation` (`local.Component`))))
  (if (== (`ActorComponent.GetOwner` Component) self)
    (`|ExecutionSequence`
      (:`then_0`
        (bind _asstatic_mesh_component (cast `StaticMeshComponent` (`local.Component`)))
        (`|ExecutionSequence`
          (:`then_0`
            (`PrimitiveComponent.SetCollisionProfileName` (`self.Mesh`) "Ragdoll" true)
            (`PrimitiveComponent.SetCollisionProfileName` (`self.CapsuleComponent`) "Spectator" true))
          (:`then_1`
            (`self.SliceStaticMesh` _asstatic_mesh_component _returnvalue _location)
            (`PrimitiveComponent.SetSimulatePhysics` (`self.Mesh`) true))))
      (:`then_1`
        (bind _asprocedural_mesh_component (cast `ProceduralMeshComponent` (`local.Component`)))
        (`self.SliceProcedualMesh` _asprocedural_mesh_component _returnvalue _location)))))

(fn `SliceProcedualMesh`
  (params (ProcMesh :type "ProceduralMeshComponent Object Reference") (Normal :type "Vector Structure") (Point :type "Vector Structure"))
  (locals (ParentMesh :type "SceneComponent Object Reference") (ChildMeshs :type "Array of SceneComponent Object Reference") (SliceNormal :type "Vector Structure" :default (0.0 0.0 0.0)) (OtherHalfProcMesh :type "ProceduralMeshComponent Object Reference"))
  (bind _procmesh (`local.ProcMesh`))
  (bind _childmeshs (`local.ChildMeshs`))
  (set `local.SliceNormal` (`local.Normal`))
  (`|ExecutionSequence`
    (:`then_0`
      (set `local.ParentMesh` (`SceneComponent.GetAttachParent` (`local.ProcMesh`)))
      (set `local.ChildMeshs` (`SceneComponent.GetChildrenComponents` (`local.ProcMesh`) false)))
    (:`then_1`
      (if (not (`.bSuccess` (cast `SkeletalMeshComponent` (`local.ParentMesh`) :!pure true)))
        (if (not (> (`KismetMathLibrary.Dot_VectorVector` (`local.Normal`) (`KismetMathLibrary.GetDirectionUnitVector` (`KismetSystemLibrary.GetComponentBounds` _procmesh) (`SceneComponent.K2_GetComponentLocation` _procmesh))) 0.0))
          (set `local.SliceNormal` (* (`local.Normal`) -1.0)))
        (elif (`KismetArrayLibrary.Array_IsNotEmpty` _childmeshs)
          (if (not (> (`KismetMathLibrary.Dot_VectorVector` (`local.Normal`) (`KismetMathLibrary.GetDirectionUnitVector` (`SceneComponent.K2_GetComponentLocation` (`|GetArrayItem` _childmeshs)) (`SceneComponent.K2_GetComponentLocation` (`local.ProcMesh`)))) 0.0))
            (set `local.SliceNormal` (* (`local.Normal`) -1.0)))
          (elif (`.bSuccess` (cast `SkeletalMeshComponent` (`local.ParentMesh`) :!pure true))
            (if (>= (`KismetMathLibrary.Dot_VectorVector` (`local.Normal`) (`KismetMathLibrary.GetDirectionUnitVector` (`KismetSystemLibrary.GetComponentBounds` (`local.ProcMesh`)) (`SceneComponent.GetSocketLocation` (`self.Mesh`) (`SceneComponent.GetAttachSocketName` (`local.ProcMesh`))))) 0.0)
              (set `local.SliceNormal` (* (`local.Normal`) -1.0)))))))
    (:`then_2`
      (bind _outotherhalfprocmesh (`KismetProceduralMeshLibrary.SliceProceduralMesh` (`local.ProcMesh`) (`local.Point`) (`local.SliceNormal`) true "CreateNewSectionForCap" "/Engine/EngineDebugMaterials/VertexColorViewMode_RedOnly.VertexColorViewMode_RedOnly"))
      (bind _output_get (set `local.OtherHalfProcMesh` _outotherhalfprocmesh))
      (`PrimitiveComponent.SetCollisionEnabled` _output_get "QueryAndPhysics")
      (`PrimitiveComponent.SetSimulatePhysics` (`local.OtherHalfProcMesh`) true)
      (for _array_element (`local.ChildMeshs`)
        (`SceneComponent.K2_AttachToComponent` _array_element (`local.OtherHalfProcMesh`) "None" "KeepWorld" "KeepWorld" "KeepWorld" true)))))

(fn `SliceStaticMesh`
  (params (BoneMesh :type "StaticMeshComponent Object Reference") (Normal :type "Vector Structure") (Point :type "Vector Structure"))
  (locals (ProcMesh :type "ProceduralMeshComponent Object Reference") (SliceMeshName :type Name :default "None") (ParentMesh :type "StaticMeshComponent Object Reference") (OtherHalfProcMesh :type "ProceduralMeshComponent Object Reference") (SlicePlaneNormal :type "Vector Structure") (ParentBoneName :type Name :default "None") (AttachedProcMeshs :type "Array of SceneComponent Object Reference"))
  (bind (_value _returnvalue) (`BlueprintMapLibrary.Map_Find` (`self.ProcMeshMap`) (`local.ParentBoneName`)))
  (`|ExecutionSequence`
    (:`then_0`
      (bind _returnvalue_2 (`AddComponent|NODE_AddProceduralMeshComponent-1` :`bManualAttachment` true))
      (set `local.ProcMesh` _returnvalue_2)
      (`KismetProceduralMeshLibrary.CopyProceduralMeshFromStaticMeshComponent` (`local.BoneMesh`) 0 (`local.ProcMesh`))
      (bind _vertices (`KismetProceduralMeshLibrary.GetSectionFromStaticMesh` (`StaticMeshComponent.StaticMesh` (`local.BoneMesh`))))
      (`ProceduralMeshComponent.AddCollisionConvexMesh` (`local.ProcMesh`) _vertices)
      (bind _output_get (set `local.SliceMeshName` (`KismetStringLibrary.Conv_StringToName` (`KismetStringLibrary.ToLower` (`KismetSystemLibrary.GetObjectName` (`local.BoneMesh`))))))
      (bind (_returnvalue_3 _parentbonename) (`self.FindParentBoneMesh` _output_get))
      (set `local.ParentMesh` _returnvalue_3)
      (set `local.ParentBoneName` _parentbonename))
    (:`then_1`
      (if (>= (`KismetMathLibrary.Dot_VectorVector` (`KismetMathLibrary.GetDirectionUnitVector` (`SceneComponent.GetSocketLocation` (`self.Mesh`) (`KismetStringLibrary.Conv_StringToName` (`KismetStringLibrary.ToLower` (`KismetSystemLibrary.GetObjectName` (`local.BoneMesh`))))) (`KismetSystemLibrary.GetComponentBounds` (`local.BoneMesh`))) (`local.Normal`)) 0.0)
        (set `local.SlicePlaneNormal` (`local.Normal`))
        (else
          (set `local.SlicePlaneNormal` (* (`local.Normal`) -1.0)))))
    (:`then_2`
      (set `local.AttachedProcMeshs` (`SceneComponent.GetChildrenComponents` (`local.BoneMesh`) false))
      (`ActorComponent.K2_DestroyComponent` (`local.BoneMesh`))
      (`PrimitiveComponent.SetCollisionEnabled` (`local.ProcMesh`) "QueryOnly")
      (`BlueprintMapLibrary.Map_Add` (`self.ProcMeshMap`) (`local.SliceMeshName`) (`local.ProcMesh`))
      (`SceneComponent.K2_AttachToComponent` (`local.ProcMesh`) (`self.Mesh`) (`local.SliceMeshName`) "SnapToTarget" "SnapToTarget" "SnapToTarget" true)
      (bind _outotherhalfprocmesh (`KismetProceduralMeshLibrary.SliceProceduralMesh` (`local.ProcMesh`) (`local.Point`) (`local.SlicePlaneNormal`) true "CreateNewSectionForCap" "/Engine/EngineDebugMaterials/VertexColorViewMode_RedOnly.VertexColorViewMode_RedOnly"))
      (bind _output_get_2 (set `local.OtherHalfProcMesh` _outotherhalfprocmesh))
      (`PrimitiveComponent.SetCollisionEnabled` _output_get_2 "QueryOnly")
      (`/Engine/EditorBlueprintResources/StandardMacros.IsValid` (`local.ParentMesh`)
        (:`Is Valid`
          (`SceneComponent.K2_AttachToComponent` (`local.OtherHalfProcMesh`) (`local.ParentMesh`) "None" "KeepWorld" "KeepWorld" "KeepWorld" true)
          (for _array_element (`local.AttachedProcMeshs`) :!label _label
            (`SceneComponent.K2_AttachToComponent` _array_element (`local.ProcMesh`) "None" "KeepWorld" "KeepWorld" "KeepWorld" true))
          (`SkeletalMeshComponent.BreakConstraint` (`self.Mesh`) (0.0 0.0 0.0) (0.0 0.0 0.0) (`local.SliceMeshName`)))
        (:`Is Not Valid`
          (if _returnvalue
            (`SceneComponent.K2_AttachToComponent` (`local.OtherHalfProcMesh`) _value "None" "KeepWorld" "KeepWorld" "KeepWorld" true)
            (goto _label)
            (else
              (`PrimitiveComponent.SetCollisionEnabled` (`local.OtherHalfProcMesh`) "QueryAndPhysics")
              (`PrimitiveComponent.SetSimulatePhysics` (`local.OtherHalfProcMesh`) true))))))))

(fn `UserConstructionScript`)